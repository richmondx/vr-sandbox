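; CurveActor_BP is an actor that draws a curve point by point along a spline, as either mesh segments or surface decals.
; AddSplinePointMesh adds a shadowless spline mesh one point behind the newest, using BaseMaterial_2 and ignoring its Material and Mesh inputs.
; AddSplinePointDecal adds a point at the stored Hit, then fills the newest segment with overlapping decals spaced by Scale, oriented to the hit normal.
; The construction-script rebuild loop is disconnected.
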(fn `AddSplinePoint_Decal`
  (params (DecalMaterial :type "MaterialInstance Object Reference") (Hit :type "HitResult Structure") (Scale :type "Float (double-precision)"))
  (locals (DecalSpacing :type "Float (double-precision)" :default 3.0))
  (bind _returnvalue (`KismetMathLibrary.MakeVector` 2.0 Scale Scale))
  (bind _returnvalue_2 (/ Scale 1.7))
  (bind _returnvalue_3 (`KismetMathLibrary.Conv_VectorToRotator` Hit_Normal))
  (bind _spline (`self.Spline`))
  (bind _returnvalue_4 (`SplineComponent.GetNumberOfSplinePoints` _spline))
  (bind _returnvalue_5 (`SplineComponent.GetDistanceAlongSplineAtSplinePoint` _spline (- _returnvalue_4 2)))
  (`SplineComponent.AddSplinePoint` _spline Hit_Location "World" true)
  (bind _returnvalue_6 (`GameplayStatics.SpawnDecalAttached` DecalMaterial _returnvalue Hit_HitComponent "None" Hit_Location _returnvalue_3 "KeepWorldPosition"))
  (for _index (range 1 (+ (`KismetMathLibrary.FTrunc` (/ (- (`SplineComponent.GetDistanceAlongSplineAtSplinePoint` _spline (- _returnvalue_4 1)) _returnvalue_5) _returnvalue_2)) 1))
    (bind _returnvalue_location (`KismetMathLibrary.BreakTransform` (`SplineComponent.GetTransformAtDistanceAlongSpline` _spline (+ (* _index _returnvalue_2) _returnvalue_5) "World" true)))
    (bind _returnvalue_7 (`GameplayStatics.SpawnDecalAttached` DecalMaterial _returnvalue Hit_HitComponent "None" _returnvalue_location _returnvalue_3 "KeepWorldPosition"))))

(fn `AddSplinePoint_Mesh`
  (params (Position :type "Vector Structure") (Material :type "MaterialInstance Object Reference") (Mesh :type "StaticMesh Object Reference") (Scale :type "Float (double-precision)"))
  (bind _returnvalue (`KismetMathLibrary.MakeVector2D` Scale Scale))
  (bind _spline (`self.Spline`))
  (bind _returnvalue_2 (`SplineComponent.GetNumberOfSplinePoints` _spline))
  (bind (_location _tangent) (`SplineComponent.GetLocationAndTangentAtSplinePoint` _spline (- _returnvalue_2 2) "Local"))
  (bind (_location_2 _tangent_2) (`SplineComponent.GetLocationAndTangentAtSplinePoint` _spline (- _returnvalue_2 3) "Local"))
  (`SplineComponent.AddSplinePoint` _spline Position "World" true)
  (bind _returnvalue_3 (`AddComponent|NODE_AddSplineMeshComponent-0`))
  (`SplineMeshComponent.SetStartScale` _returnvalue_3 _returnvalue true)
  (`SplineMeshComponent.SetEndScale` _returnvalue_3 _returnvalue true)
  (`PrimitiveComponent.SetCastShadow` _returnvalue_3 false)
  (`PrimitiveComponent.SetMaterial` _returnvalue_3 0 "/Game/FirstPerson/Meshes/BaseMaterial_2.BaseMaterial_2")
  (`SplineMeshComponent.SetStartAndEnd` _returnvalue_3 _location_2 _tangent_2 _location _tangent true))

(fn `UserConstructionScript`)