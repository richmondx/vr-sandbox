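; Action controller for a paint-and-build tool with three modes: wall decal painting, mid-air mesh drawing and physics mesh spawning.
; FireAction feeds decal trace hits or points ahead of an arrow into a spawned SplineActor, or spawns one mesh until EndAction resets.
; BeginPlay builds decal materials for every color and mask pair.
; Brush events adjust size and indices, but wall material selection is unwired and space drawing uses a fixed material.
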(event `self.ReceiveBeginPlay`
  (`self.Init Materials`))

(event `self.ReceiveTick`
  (params (DeltaSeconds :type "Float (single-precision)"))
  ;[1 0.7459 0.1808] Tick
  (`self.Rotate Material Sphere` 1.0))

(event `FireAction`
  (bind _splineactor_ref (`self.SplineActor Ref`))
  ;[1 0.007701 0] Event fire
  (`self.Rotate Material Sphere` 3.0)
  (switch `int` (`self.Mode`)
    (:`0`
      (`/Engine/EditorBlueprintResources/StandardMacros.IsValid` _splineactor_ref
        (:`Is Valid`
          _)
        (:`Is Not Valid`
          (`self.CreateCurve`)))
      (`self.WallPaint`))
    (:`1`
      (`/Engine/EditorBlueprintResources/StandardMacros.IsValid` _splineactor_ref
        (:`Is Valid`
          _)
        (:`Is Not Valid`
          (`self.CreateCurve`)))
      (`KismetSystemLibrary.Delay` 0.03)
      (`self.SpaceDraw`))
    (:`2`
      (`/Engine/EditorBlueprintResources/StandardMacros.DoOnce` false :!label _label
        (:`Completed`
          (`self.SpawnMesh`))))))

(event `ChangeMode`
  (params (NewParam :type Integer))
  ;[1 0.2353 0.9005] Change mode
  (set `self.Mode` NewParam))

(event `EndAction`
  ;[0.4075 0.2387 1] End action - cleanup
  (set `self.CurveActorRef` null)
  (set `self.SplineActor Ref` null)
  (goto _label :!via `Reset`))

(event `Change Brush Size`
  (params (`Size Increase` :type "Float (double-precision)"))
  (switch `int` (`self.Mode`)
    (:`0`
      (bind _output_get (set `self.Brush Size Wall` (+ (`self.Brush Size Wall`) `Size Increase`)))
      (`KismetSystemLibrary.PrintString` (`KismetStringLibrary.BuildString_Double` "" "WALL Brush size:" _output_get)))
    (:`1`
      (bind _output_get_2 (set `self.Brush Size Space` (+ (`self.Brush Size Space`) (* `Size Increase` 0.3))))
      (`KismetSystemLibrary.PrintString` (`KismetStringLibrary.BuildString_Double` "" "SPACE Brush size:" _output_get_2)))))

(event `Change Brush`
  (params (`Color Index+/-` :type Integer) (`Brush Index+/-` :type Integer))
  (bind _spacepaintmaterials (`self.SpacePaintMaterials`))
  (switch `int` (`self.Mode`)
    (:`0`
      (bind _output_get (set `self.WallPaintColorIndex` (+ (`self.WallPaintColorIndex`) `Color Index+/-`)))
      (set `self.WallPaintBrushIndex` (+ (`self.WallPaintBrushIndex`) `Brush Index+/-`)))
    (:`1`
      (bind _output_get_2 (set `self.SpacePaintMatIndex` (+ (`self.SpacePaintMatIndex`) `Color Index+/-`)))
      (set `self.M_WallPaint Inst` (`|GetArrayItem` _spacepaintmaterials (`KismetMathLibrary.Clamp` _output_get_2 0 (- (`KismetArrayLibrary.Array_Length` _spacepaintmaterials) 1)))))))

(fn `CreateCurve`
  (bind _arrowref (`self.ArrowRef`))
  (bind (_returnvalue_location _returnvalue_rotation) (`KismetMathLibrary.BreakTransform` (`SceneComponent.K2_GetComponentToWorld` _arrowref)))
  (bind _returnvalue (`|SpawnActorFromClass` "/Script/DiplomaVr.SplineActor" (`KismetMathLibrary.MakeTransform` (+ _returnvalue_location (* (`SceneComponent.GetForwardVector` _arrowref) 200)) _returnvalue_rotation) "Undefined" "OverrideRootScale" (`self.GetOwner`) null))
  (set `self.SplineActor Ref` _returnvalue))

(fn `Init Materials`
  (locals (Colors :type "Array of LinearColor Structure") (DecalMasks :type "Array of Texture Object Reference"))
  (for _array_element (`local.Colors`)
    (for _array_element_2 (`local.DecalMasks`)
      (bind _returnvalue (`KismetMaterialLibrary.CreateDynamicMaterialInstance` "/Game/ActionController/Materials/M_DecalBase.M_DecalBase"))
      (`MaterialInstanceDynamic.SetVectorParameterValue` _returnvalue "DecalColor" _array_element)
      (`MaterialInstanceDynamic.SetTextureParameterValue` _returnvalue "DecalMaskTexture" _array_element_2)
      (`KismetArrayLibrary.Array_Add` (`self.WallPaintMaterials`) _returnvalue)))
  (set `self.M_WallPaint Inst` (`|GetArrayItem` (`self.WallPaintMaterials`))))

(fn `Rotate Material Sphere`
  (params (Speed :type "Float (double-precision)"))
  (bind _materialsphere (`self.MaterialSphere`))
  (bind (_returnvalue_location _returnvalue_rotation) (`KismetMathLibrary.BreakTransform` (`SceneComponent.GetRelativeTransform` _materialsphere)))
  (`/Engine/EditorBlueprintResources/StandardMacros.IsValid` _materialsphere
    (:`Is Valid`
      (`SceneComponent.K2_SetRelativeRotation` _materialsphere (`KismetMathLibrary.ComposeRotators` _returnvalue_rotation (* (`KismetMathLibrary.MakeRotator` 1.0 0.2 0.7) Speed)) false false))))

(fn `SpaceDraw`
  (bind _splineactor_ref (`self.SplineActor Ref`))
  (bind _arrowref (`self.ArrowRef`))
  (`/Engine/EditorBlueprintResources/StandardMacros.IsValid` _splineactor_ref
    (:`Is Valid`
      (`SplineActor.AddSplinePoint_Mesh` _splineactor_ref (+ (`SceneComponent.K2_GetComponentLocation` _arrowref) (* (`SceneComponent.GetForwardVector` _arrowref) 200)) "/Game/FirstPerson/Meshes/BaseMaterial_2.BaseMaterial_2" "/Game/ActionController/Meshes/Cylinder_Brush23_StaticMesh.Cylinder_Brush23_StaticMesh" (`self.Brush Size Space`)))))

(fn `SpawnMesh`
  (bind _arrowref (`self.ArrowRef`))
  (bind _returnvalue (`|SpawnActorFromClass` "/Script/DiplomaVr.MeshActor" (`KismetMathLibrary.MakeTransform` (+ (`SceneComponent.K2_GetComponentLocation` _arrowref) (* (`SceneComponent.GetForwardVector` _arrowref) 200))) "Undefined" "OverrideRootScale" null (`GameplayStatics.GetPlayerPawn` 0)))
  (bind _returnvalue_2 (`StaticMeshComponent.SetStaticMesh` (`StaticMeshActor.StaticMeshComponent` _returnvalue) (`|GetArrayItem` (`self.SpawnableMeshList`) (`self.SpawnMesh Index`))))
  (if _returnvalue_2
    (`PrimitiveComponent.SetSimulatePhysics` (`StaticMeshActor.StaticMeshComponent` _returnvalue) true)
    (`PrimitiveComponent.SetSimulatePhysics` (`StaticMeshActor.StaticMeshComponent` _returnvalue) true)
    (set `MeshActor.bIsSpawned` true _returnvalue)))

(fn `WallPaint`
  (bind _arrowref (`self.ArrowRef`))
  (bind _splineactor_ref (`self.SplineActor Ref`))
  (bind _returnvalue (`SceneComponent.K2_GetComponentLocation` _arrowref))
  (bind _outhit (`KismetSystemLibrary.LineTraceSingle` _returnvalue (+ _returnvalue (* (`SceneComponent.GetForwardVector` _arrowref) 700)) "TraceTypeQuery2" true))
  (`KismetSystemLibrary.PrintString` "DRAW_Decal")
  (`/Engine/EditorBlueprintResources/StandardMacros.IsValid` _splineactor_ref
    (:`Is Valid`
      (`SplineActor.AddSplinePoint_Decal` _splineactor_ref (`self.M_WallPaint Inst`) (`self.Brush Size Wall`) _outhit))))