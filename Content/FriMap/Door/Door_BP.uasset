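; Interactive door Blueprint that swings its DoorFrame open or closed when PickUp is called, unless Disable is set.
; PickUp triggers OpenCloseDoor, which plays or reverses a timeline based on IsOpened and flips that flag when the timeline finishes.
; The timeline's OpenDoor track drives the frame's relative yaw, with IsInverted selecting a modified value for the swing.
; Drop does nothing, and both PickUp and Drop return false.
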(event `OpenClose Door`
  (bind _bisopened (`self.bIsOpened`))
  (bind _doorframe (`self.DoorFrame`))
  (bind _returnvalue (`SceneComponent.GetRelativeTransform` _doorframe))
  (if (`self.bDisable`)
    _
    (elif _bisopened
      (bind (_direction _opendoor) (`Timeline|Timeline_0` :!label _label)
        (:`Update`
          (if (`self.bIsInverted`)
            (bind _result (`/Engine/EditorBlueprintResources/StandardMacros.NegateFloat` _opendoor)
              (:`  `
                (`SceneComponent.K2_SetRelativeRotation` _doorframe (`KismetMathLibrary.MakeRotator` (.roll (.rotation _returnvalue)) (.pitch (.rotation _returnvalue)) _result) false false)))
            (else
              (`SceneComponent.K2_SetRelativeRotation` _doorframe (`KismetMathLibrary.MakeRotator` (.roll (.rotation _returnvalue)) (.pitch (.rotation _returnvalue)) _opendoor) false false))))
        (:`Finished`
          (set `self.bIsOpened` (not _bisopened))))
      (else
        (goto _label :!via `Reverse`)))))

(fn `Drop`
  (returns (ReturnValue :type Boolean))
  (return false))

(fn `PickUp`
  (params (attachTo :type "SceneComponent Object Reference"))
  (returns (ReturnValue :type Boolean))
  (`self.OpenClose Door`)
  (return false))

(fn `UserConstructionScript`)